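; Level manager actor that runs the game flow from start menu through play to game over.
; BeginPlay shows the start menu with a self-reference and caches the player pawn.
; StartGame and GameOver toggle play state, input mode and cursor; GameOver also zeroes level speed and shows its widget.
; The LevelBounds box, configured in the construction script, passes overlapping actors to their reported parent through SpawnActorHitBound for obstacle spawning.
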(event `self.ReceiveBeginPlay`
  ;[1 1 1] Стартовое меню
  (bind _returnvalue (`|CreateWidget` "/Game/Blueprint/UI/StartMenu.StartMenu_C" null self))
  (`UserWidget.AddToViewport` _returnvalue 0)
  ;[1 1 1] Запуск игрока
  (bind _asmy_pawn_base_bp (cast `/Game/Blueprint/Game/MyPawnBase_BP` (`GameplayStatics.GetPlayerPawn` 0)))
  (set `self.PlayerRef` _asmy_pawn_base_bp))

(event `self.LevelBounds.OnComponentBeginOverlap`
  (params (OverlappedComponent :type "PrimitiveComponent Object Reference") (OtherActor :type "Actor Object Reference") (OtherComp :type "PrimitiveComponent Object Reference") (OtherBodyIndex :type Integer) (bFromSweep :type Boolean) (SweepResult :type "HitResult Structure (by ref)"))
  ;[1 1 1] Спаун препятствий, проверка столкновений
  (bind _parent (message `/Game/Blueprint/Misc/BPI_Spawnable.ReturnParent` OtherActor))
  (`/Engine/EditorBlueprintResources/StandardMacros.IsValid` _parent
    (:`Is Valid`
      (`/Game/Blueprint/Spawner/SpawnerBase.SpawnActorHitBound` _parent OtherActor))))

(fn `GameOver`
  (bind _returnvalue (`GameplayStatics.GetPlayerController` 0))
  ;[1 1 1] Игра останавливается, создается виджет о конце игры
  (set `self.LevelSpeed` 0.0)
  (set `self.isPlaying` false)
  (bind _returnvalue_2 (`|CreateWidget` "/Game/Blueprint/UI/GameOver.GameOver_C" null null))
  ;[1 1 1] Курсор возвращается
  (`UserWidget.AddToViewport` _returnvalue_2 0)
  (`WidgetBlueprintLibrary.SetInputMode_UIOnlyEx` _returnvalue null)
  (set `PlayerController.bShowMouseCursor` true _returnvalue))

(fn `StartGame`
  (bind _returnvalue (`GameplayStatics.GetPlayerController` 0))
  ;[1 1 1] В начале курсор убирается, сразу начинается игра
  (set `self.isPlaying` true)
  (`WidgetBlueprintLibrary.SetInputMode_GameOnly` _returnvalue)
  (set `PlayerController.bShowMouseCursor` false _returnvalue)
  (`/Game/Blueprint/Game/MyPawnBase_BP.GameStarted` (`self.PlayerRef`)))

(fn `UserConstructionScript`
  (bind _levelbounds (`self.LevelBounds`))
  ;[1 1 1] Размещение игрока
  (`BoxComponent.SetBoxExtent` _levelbounds (`self.OutOfBoundBoxScale`) true)
  (`SceneComponent.K2_SetWorldLocation` _levelbounds (`self.OutOfBoundBoxLocation`) false false))