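; Base player pawn for a lane-based game, stepping left and right between lanes while the level manager reports play.
; Initialise takes lane count and width from that manager; timelines lerp Y per move, blocking input until finished.
; GameStarted adds the trail and HUD; HitObst spawns fire, blends to the EndCam-tagged camera and destroys player and trail components.
; Touch swipe detection only runs at BeginPlay with empty branches, and jump logic is disconnected.
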(event `self.ReceiveBeginPlay`
  (bind (_locationx _locationy) (`PlayerController.GetInputTouchState` (`GameplayStatics.GetPlayerController` 0) "Touch1"))
  (bind _returnvalue (`KismetMathLibrary.MakeVector2D` _locationx _locationy))
  (bind (_x _y) (`KismetMathLibrary.BreakVector2D` (- (`self.TouchStart`) (`self.TouchEnd`))))
  (`|ExecutionSequence`
    (:`then_0`
      (if (`self.isPressed`)
        (if (> (`KismetMathLibrary.VSize2D` (- (`self.TouchStart`) _returnvalue)) 100.0)
          (`/Engine/EditorBlueprintResources/StandardMacros.DoOnce` false :!label _label
            (:`Completed`
              (set `self.TouchEnd` _returnvalue)
              (if (> (`KismetMathLibrary.Abs` _x) (`KismetMathLibrary.Abs` _y))
                (if (> _x 0.0)
                  _)
                (elif (> _y 0.0)
                  _)))))))
    (:`then_1`
      ;[1 1 1] Начало игрв
      (`self.Initialise`))))

(event `InputAction|Left`
  (params (Key :type "Key Structure"))
  (bind (_returnvalue_x _returnvalue_y) (`KismetMathLibrary.BreakVector` (`self.K2_GetActorLocation`)))
  (bind (_returnvalue_x_2 _returnvalue_y_2 _returnvalue_z) (`KismetMathLibrary.BreakVector` (`self.K2_GetActorLocation`)))
  (:`Pressed`
    (if (`/Game/Blueprint/Game/LevelManager.isPlaying` (`self.LevelManRef`))
      (if (not (<= (`self.CurrentLane`) 1))
        ;[1 1 1] Передвижение влево
        (if (not (`self.bMoving`))
          (set `self.bMoving` true)
          (set `self.TargetPosition` (- _returnvalue_y (`self.Lane Width`)))
          (bind (_direction _move) (`Timeline|MoveLeft` :!via `PlayFromStart`)
            (:`Update`
              (`self.K2_SetActorLocation` (`KismetMathLibrary.MakeVector` _returnvalue_x_2 (`KismetMathLibrary.Lerp` _returnvalue_y_2 (`self.TargetPosition`) _move) _returnvalue_z)))
            (:`Finished`
              (set `self.bMoving` false)
              (`/Engine/EditorBlueprintResources/StandardMacros.DecrementInt` (`self.CurrentLane`)))))))))

(event `InputAction|Finger`
  (params (Key :type "Key Structure"))
  (bind (_locationx _locationy) (`PlayerController.GetInputTouchState` (`GameplayStatics.GetPlayerController` 0) "Touch1"))
  (:`Pressed`
    (set `self.isPressed` true)
    (set `self.TouchStart` (`KismetMathLibrary.MakeVector2D` _locationx _locationy)))
  (:`Released`
    (set `self.isPressed` false)
    (goto _label :!via `Reset`)))

(event `InputAction|Right`
  (params (Key :type "Key Structure"))
  (bind (_returnvalue_x _returnvalue_y _returnvalue_z) (`KismetMathLibrary.BreakVector` (`self.K2_GetActorLocation`)))
  (bind (_returnvalue_x_2 _returnvalue_y_2) (`KismetMathLibrary.BreakVector` (`self.K2_GetActorLocation`)))
  (:`Pressed`
    ;[1 1 1] Проверка нажата ли самая правая
    (if (`/Game/Blueprint/Game/LevelManager.isPlaying` (`self.LevelManRef`))
      (if (not (== (`self.CurrentLane`) (`/Game/Blueprint/Game/LevelManager.NumOfLane` (`self.LevelManRef`))))
        ;[1 1 1] Передвижение вправо
        (if (not (`self.bMoving`))
          (set `self.bMoving` true)
          (set `self.TargetPosition` (+ _returnvalue_y_2 (`self.Lane Width`)))
          (bind (_direction _move) (`Timeline|MoveRight` :!via `PlayFromStart`)
            (:`Update`
              (`self.K2_SetActorLocation` (`KismetMathLibrary.MakeVector` _returnvalue_x (`KismetMathLibrary.Lerp` _returnvalue_y (`self.TargetPosition`) _move) _returnvalue_z)))
            (:`Finished`
              (set `self.bMoving` false)
              (`/Engine/EditorBlueprintResources/StandardMacros.IncrementInt` (`self.CurrentLane`)))))))))

(event `InputAction|Jump`
  (params (Key :type "Key Structure"))
  ;[1 1 1] Прыжок
)

(fn `GameStarted`
  ;[1 1 1] Появление хвоста на старте
  (`ParticleSystemComponent.SetTemplate` (`self.ParticleSystem`) "/Game/InfinityBladeEffects/Effects/FX_Mobile/Fire/combat/P_AOE_Fire_CircleAttack.P_AOE_Fire_CircleAttack")
  ;[1 1 1] Виджет подсчета очков
  (bind _returnvalue (`|CreateWidget` "/Game/Blueprint/UI/HUD.HUD_C"))
  (`UserWidget.AddToViewport` _returnvalue 0))

(fn `HitObst`
  ;[1 1 1] Расположение хвоста
  (`GameplayStatics.SpawnEmitterAtLocation` "/Game/InfinityBladeEffects/Effects/FX_Mobile/Fire/combat/P_AOE_Fire_CircleAttack.P_AOE_Fire_CircleAttack" (`self.K2_GetActorLocation`))
  ;[1 1 1] Поднятие камеры во время смерти
  (`PlayerController.SetViewTargetWithBlend` (`GameplayStatics.GetPlayerController` 0) (`self.EndCamRef`) 1.0 "VTBlend_Linear" 0.0 false)
  ;[1 1 1] Исчезновение игрока
  (`ActorComponent.K2_DestroyComponent` (`self.Player`))
  ;[1 1 1] Исчезновение хвоста
  (`ActorComponent.K2_DestroyComponent` (`self.ParticleSystem`)))

(fn `Initialise`
  (bind (_levelmanag _levelmanfound) (`/Game/Blueprint/Lib/BPF_Lib.GetLevelManag`))
  ;[1 1 1] Перемещение по линиям
  (if _levelmanfound
    (set `self.LevelManRef` _levelmanag)
    (set `self.CurrentLane` (+ (/ (`/Game/Blueprint/Game/LevelManager.NumOfLane` (`self.LevelManRef`)) 2) 1))
    (set `self.Lane Width` (`/Game/Blueprint/Game/LevelManager.LaneWidth` (`self.LevelManRef`)))
    ;[1 1 1] Смещение камеры после смерти
    (bind _outactors (`GameplayStatics.GetAllActorsWithTag` "EndCam"))
    (set `self.EndCamRef` (`|GetArrayItem` _outactors))
    (else
      (`KismetSystemLibrary.PrintString` " No LevelMan Found"))))

(fn `UserConstructionScript`)