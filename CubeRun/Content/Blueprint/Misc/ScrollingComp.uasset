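; ScrollingComp is a component that scrolls its owning actor at the level's speed during play.
; It caches the level manager on BeginPlay if one is found.
; Each Tick, while the manager is playing, it moves the owner without sweep by forward vector times LevelSpeed and delta time.
; The world-space forward vector is applied as a local offset, so the owner's rotation affects the direction twice.
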(event `self.ReceiveBeginPlay`
  (bind (_levelmanag _levelmanfound) (`/Game/Blueprint/Lib/BPF_Lib.GetLevelManag`))
  (if _levelmanfound
    (set `self.LevelManRef` _levelmanag)))

(event `self.ReceiveTick`
  (params (DeltaSeconds :type "Float (single-precision)"))
  (bind _levelmanref (`self.LevelManRef`))
  (set `self.Delta Seconds` DeltaSeconds)
  (`/Engine/EditorBlueprintResources/StandardMacros.IsValid` _levelmanref
    (:`Is Valid`
      (if (`/Game/Blueprint/Game/LevelManager.isPlaying` _levelmanref)
        (bind _output_get (set `self.Movement` (* (* (`Actor.GetActorForwardVector` (`self.GetOwner`)) (`/Game/Blueprint/Game/LevelManager.LevelSpeed` (`self.LevelManRef`))) (`self.Delta Seconds`))))
        (`Actor.K2_AddActorLocalOffset` (`self.GetOwner`) _output_get false false)))))