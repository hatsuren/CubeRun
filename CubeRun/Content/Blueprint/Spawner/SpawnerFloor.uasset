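; Floor spawner Blueprint that builds an endless road from a recycled row of tiles along the X axis.
; On BeginPlay it spawns the first tile at its own location, measures its X bounds, then chains further tiles behind one another up to ActorReqCount.
; SpawnActorHitBound moves an out-of-bounds tile, after a tiny delay, one tile length beyond RearTile and makes it the new RearTile, reusing actors instead of spawning more.
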(event `self.ReceiveBeginPlay`
  (bind (_returnvalue_x _returnvalue_y) (`KismetMathLibrary.BreakVector` (`self.K2_GetActorLocation` (`self.RearTile`))))
  (`parent.ReceiveBeginPlay`)
  (for _index (range (+ (`self.ActorReqCount`) 1))
    (if (== _index 0)
      ;[1 1 1] Спаун первой площадки
      (bind _returnvalue (`self.SpawnActor`))
      (set `self.RearTile` _returnvalue)
      (set `self.TileSize` (* (.x (`.BoxExtent` (`self.GetActorBounds` _returnvalue false false))) 2.0))
      (`self.K2_SetActorLocation` (`self.RearTile`) (`self.K2_GetActorLocation`) false false)
      (else
        (bind _returnvalue_2 (`self.SpawnActor`))
        (`self.K2_SetActorLocation` _returnvalue_2 (`KismetMathLibrary.MakeVector` (+ _returnvalue_x (`self.TileSize`)) _returnvalue_y) false false)
        (set `self.RearTile` _returnvalue_2)))))

(event `self.SpawnActorHitBound`
  (params (OutOfBoundsActor :type "Actor Object Reference"))
  (bind (_returnvalue_x _returnvalue_y _returnvalue_z) (`KismetMathLibrary.BreakVector` (`self.K2_GetActorLocation` (`self.RearTile`))))
  ;[1 1 1] Спаун Дороги вперед
  (`KismetSystemLibrary.Delay` 0.01)
  (`self.K2_SetActorLocation` OutOfBoundsActor (`KismetMathLibrary.MakeVector` (+ _returnvalue_x (`self.TileSize`)) _returnvalue_y _returnvalue_z) false false)
  (set `self.RearTile` OutOfBoundsActor))

(fn `UserConstructionScript`
  (`parent.UserConstructionScript`))