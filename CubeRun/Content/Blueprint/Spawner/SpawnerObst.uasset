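; Obstacle spawner Blueprint that places obstacles at its own location at random intervals during play.
; On BeginPlay it looks up the level manager and, if found, starts a self-rescheduling delay loop that repeats while the level is playing.
; Each cycle gets an actor from the parent class's SpawnActor and teleport-free moves it to the spawner.
; Spawned actors reported as out of bounds are destroyed.
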(event `self.ReceiveBeginPlay`
  (bind (_levelmanag _levelmanfound) (`/Game/Blueprint/Lib/BPF_Lib.GetLevelManag`))
  (if _levelmanfound
    (set `self.Level ManagRef` _levelmanag)
    (`self.LineUpNextObstSpawn`)))

(event `LineUpNextObstSpawn`
  (`KismetSystemLibrary.Delay` (`KismetMathLibrary.RandomFloatInRange` (`self.MinDelay`) (`self.MaxDelay`)))
  (`self.PlaceObst`)
  (if (`/Game/Blueprint/Game/LevelManager.isPlaying` (`self.Level ManagRef`))
    (`self.LineUpNextObstSpawn`)))

(event `self.SpawnActorHitBound`
  (params (OutOfBoundsActor :type "Actor Object Reference"))
  (`self.K2_DestroyActor` OutOfBoundsActor))

(fn `PlaceObst`
  (bind _returnvalue (`self.SpawnActor`))
  (`self.K2_SetActorLocation` _returnvalue (`self.K2_GetActorLocation`) false false))

(fn `SpawnActor`
  (returns (ReturnValue :type "Actor Object Reference"))
  (bind _returnvalue (`parent.SpawnActor`))
  (return _returnvalue))

(fn `UserConstructionScript`
  (`parent.UserConstructionScript`))